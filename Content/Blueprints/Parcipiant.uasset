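; Parcipiant is a dialogue participant Blueprint that stores story progress for a narrative game, such as door, key, axe, paper and clue (Uliki) states.
; Name-based switches read and write these integer variables, with only the clue counter supporting delta changes.
; The participant name comes from the GameInstances object, and dialogue events are saved to EndGameEvent before passing through a switch.
; Conditions and bool, float and name accessors are stubs.
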(fn ConstructionScript)

(fn CheckCondition
  (params (ConditionName :type Name%20%28by%20ref%29 :default "None"))
  (return false))

(fn GetBoolValue
  (params (ValueName :type Name%20%28by%20ref%29 :default "None"))
  (return false))

(fn GetFloatValue
  (params (ValueName :type Name%20%28by%20ref%29 :default "None"))
  (return 0.0))

(fn GetIntValue
  (params (ValueName :type Name%20%28by%20ref%29 :default "None"))
  (switch name ValueName
    (:Default
      (return 0))
    (:VisDoor
      (return (Variables|Default|GetVisDoor)))
    (:KeyFind
      (return (Variables|Default|GetKeyFind)))
    (:CloseDoor
      (return (Variables|Default|GetCloseDoor)))
    (:Bush
      (return (Variables|Default|GetBush)))
    (:SecretRoom
      (return (Variables|Default|GetSecretRoom)))
    (:GetAxe
      (return (Variables|Default|GetGetAxe)))
    (:Paper
      (return (Variables|Default|GetPaper)))
    (:Uliki
      (return (Variables|Default|GetUliki)))
    (:Ulika1
      (return (Variables|Default|GetUlika1)))
    (:Ulika2
      (return (Variables|Default|GetUlika2)))))

(fn GetNameValue
  (params (ValueName :type Name%20%28by%20ref%29 :default "None"))
  (return "None"))

(fn GetParticipantDisplayName
  (params (ActiveSpeaker :type Name :default "None"))
  (return ""))

(fn GetParticipantGender
  (return "Masculine"))

(fn GetParticipantIcon
  (params (ActiveSpeaker :type Name :default "None") (ActiveSpeakerState :type Name :default "None"))
  (return 0))

(fn GetParticipantName
  (bind _asgame_instances (Utilities|Casting|CastToGameInstances (Game|GetGameInstance))
    (:then
      (return (Variables|/Game/Blueprints/GameInstances.GameInstances_C|GetParcipiantName _asgame_instances)))
    (:CastFailed
      (Development|PrintString "Что-то не так с именем повествователя"))))

(fn ModifyBoolValue
  (params (ValueName :type Name%20%28by%20ref%29 :default "None") (bNewValue :type Boolean))
  (return bNewValue))

(fn ModifyFloatValue
  (params (ValueName :type Name%20%28by%20ref%29 :default "None") (bDelta :type Boolean) (Value :type Float%20%28single-precision%29))
  (return false))

(fn ModifyIntValue
  (params (ValueName :type Name%20%28by%20ref%29 :default "None") (bDelta :type Boolean) (Value :type Integer))
  (switch name ValueName
    (:Default
      _)
    (:VisDoor
      (Variables|Default|SetVisDoor Value))
    (:KeyFind
      (Variables|Default|SetKeyFind Value))
    (:CloseDoor
      (Variables|Default|SetCloseDoor Value))
    (:Bush
      (Variables|Default|SetBush Value))
    (:SecretRoom
      (Variables|Default|SetSecretRoom Value))
    (:GetAxe
      (Variables|Default|SetGetAxe Value))
    (:Paper
      (Variables|Default|SetPaper Value))
    (:Uliki
      (if bDelta
        (Variables|Default|SetUliki (+ (Variables|Default|GetUliki) Value))
        (else
          (Variables|Default|SetUliki Value))))
    (:Ulika1
      (Variables|Default|SetUlika1 Value))
    (:Ulika2
      (Variables|Default|SetUlika2 Value)))
  (return false))

(fn ModifyNameValue
  (params (ValueName :type Name%20%28by%20ref%29 :default "None") (NameValue :type Name%20%28by%20ref%29 :default "None"))
  (return false))

(fn OnDialogueEvent
  (params (EventName :type Name%20%28by%20ref%29 :default "None"))
  (bind _output_get (Variables|Default|SetEndGameEvent EventName))
  (|SwitchDialogueCallbackEvent _output_get
    (:Default
      (return false))
    (:EndStory
      (return false))))